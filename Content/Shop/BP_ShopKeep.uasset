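; BP_ShopKeep is a shopkeeper actor that opens a shop interface when an actor tagged Player overlaps its ShopTrigger.
; The overlap blends the cached player controller's view to the shopkeeper, waits for the one-second blend, then adds WB_ShopKeepUI with itself as ShopKeepNPC.
; It then switches to UI-only input, shows the cursor and calls SetActorHiddenInGame on the controller rather than the pawn.
; Nothing here closes the shop or restores the view.
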(event OnComponentBeginOverlap(ShopTrigger)
  (params (OverlappedComponent :type Primitive%20Component%20Object%20Reference) (OtherActor :type Actor%20Object%20Reference) (OtherComp :type Primitive%20Component%20Object%20Reference) (OtherBodyIndex :type Integer) (bFromSweep :type Boolean) (SweepResult :type Hit%20Result%20Structure%20%28by%20ref%29))
  (if (Actor|ActorHasTag OtherActor "Player")
    (Game|Player|SetViewTargetwithBlend (Variables|Default|GetPlayerController) self 1.0 "VTBlend_Linear" 0.0 false)
    (Utilities|FlowControl|Delay 1.0)
    (bind _returnvalue (UserInterface|CreateWidget "/Game/Shop/WB_ShopKeepUI.WB_ShopKeepUI_C" (Variables|Default|GetPlayerController) self))
    (UserInterface|Viewport|AddtoViewport _returnvalue 0)
    (Input|SetInputModeUIOnly (Variables|Default|GetPlayerController) _returnvalue "DoNotLock" false)
    (Variables|/Script/Engine.PlayerController|SetbShowMouseCursor (Variables|Default|GetPlayerController) true)
    (Rendering|SetActorHiddenInGame (Variables|Default|GetPlayerController) true)))

(event EventBeginPlay
  (Variables|Default|SetPlayerController (Game|GetPlayerController 0)))

(fn ConstructionScript)