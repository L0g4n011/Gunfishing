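; Test Blueprint for a fishing loot table: the first E press rolls a random DropID and prints a catch.
; A DoOnce feeds a Sequence of range checks that look up rows in DT_SpawnTable.
; Only the Bass check works; Sunfish and Blue Gill sit behind false branches, and Blue Gill compares a constant and reads the Sunfish row.
; "No fish Caught" prints regardless of the result.
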(event EventBeginPlay)

(event Collision|EventActorBeginOverlap
  (params (OtherActor :type Actor%20Object%20Reference)))

(event EventTick
  (params (DeltaSeconds :type Float%20%28single-precision%29)))

(event Input|KeyboardEvents|E
  (params (Key :type Key%20Structure))
  (:Pressed
    (bind _output_get (Variables|Default|SetDropID (Math|Random|RandomIntegerinRange 0 100)))
    (Utilities|FlowControl|DoOnce false
      (:Completed
        (Utilities|FlowControl|Sequence
          (:then_0
            (Math|Float|CompareFloat (Math|Conversions|ToFloat(Integer) _output_get) 5e+01
              (:<
                (Utilities|GetDataTableRow "/Game/LootTable/DT_SpawnTable.DT_SpawnTable" "Bass"
                  (:then
                    (Development|PrintString "Caught a Bass"))))))
          (:then_1
            (Math|Float|CompareFloat (Math|Conversions|ToFloat(Integer) _output_get) 51.0
              (:>
                (if false
                  (Math|Float|CompareFloat (Math|Conversions|ToFloat(Integer) _output_get) 7e+01
                    (:<
                      (Utilities|GetDataTableRow "/Game/LootTable/DT_SpawnTable.DT_SpawnTable" "Sunfish"
                        (:then
                          (Development|PrintString "Caught a Sunfish")))))))))
          (:then_2
            (Math|Float|CompareFloat 0.0 71.0
              (:>
                (if false
                  (Math|Float|CompareFloat 0.0 8e+01
                    (:<
                      (Utilities|GetDataTableRow "/Game/LootTable/DT_SpawnTable.DT_SpawnTable" "Sunfish"
                        (:then
                          (Development|PrintString "Caught a Blue Gill")))))))))
          (:then_3
            (Development|PrintString "No fish Caught")))))))

(fn ConstructionScript)