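; BP_BoxSpawner spawns fish at random points inside its trigger box while an actor tagged Player overlaps it.
; Begin overlap starts a looping timer that spawns one fish per tick, and end overlap clears it.
; Each fish class is picked from FishtoSpawn by passing a random float through SpawnCurve and rounding the result to an index, so the curve shapes the odds.
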(event OnComponentBeginOverlap(SpawnActorsTrigger)
  (params (OverlappedComponent :type Primitive%20Component%20Object%20Reference) (OtherActor :type Actor%20Object%20Reference) (OtherComp :type Primitive%20Component%20Object%20Reference) (OtherBodyIndex :type Integer) (bFromSweep :type Boolean) (SweepResult :type Hit%20Result%20Structure%20%28by%20ref%29))
  (if (Actor|ActorHasTag OtherActor "Player")
    (bind _returnvalue (Utilities|Time|SetTimerbyEvent (delegate Custom|SpawnActorsOverTime) 1.0 true))))

(event OnComponentEndOverlap(SpawnActorsTrigger)
  (params (OverlappedComponent :type Primitive%20Component%20Object%20Reference) (OtherActor :type Actor%20Object%20Reference) (OtherComp :type Primitive%20Component%20Object%20Reference) (OtherBodyIndex :type Integer))
  (if (Actor|ActorHasTag OtherActor "Player")
    (CallFunction|StopSpawningActors)))

(event Custom|SpawnActorsOverTime
  (bind _spawnactorstrigger (Variables|Default|GetSpawnActorsTrigger))
  (Game|SpawnActorfromClass (Utilities|Array|Get(acopy) (Variables|Default|GetFishtoSpawn) (Math|Float|Round (Math|Curves|GetFloatValue (Variables|Default|GetSpawnCurve) (Math|Random|RandomFloatinRange 0.0 2.0)))) (Math|Conversions|ToTransform(Vector) (Math|Random|RandomPointinBoundingBox (Transformation|GetWorldLocation _spawnactorstrigger) (Variables|/Script/Engine.BoxComponent|GetBoxExtent _spawnactorstrigger))) "Undefined" "MultiplyWithRoot" 0 0))

(event Custom|Stop%20Spawning%20Actors
  (Utilities|Time|ClearandInvalidateTimerbyHandle (stale OnComponentBeginOverlap(SpawnActorsTrigger) _returnvalue)))

(fn ConstructionScript)