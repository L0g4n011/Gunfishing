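; BP_BlackJack is an early blackjack prototype that prints to screen instead of displaying cards.
; On BeginPlay, DealCards adds random values to the player and dealer hands, using DoOnce to run a second round.
; Printed suits and values are rolled randomly, separately from stored values.
; Hit is empty, and the uncalled CheckForWinorLose totals the player's hand but treats 21 as a loss, leaving its win branch unreachable.
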(event Custom|DealCards
  (bind _returnvalue (Math|Random|RandomIntegerinRange 0 12))
  (bind _returnvalue_2 (Math|Random|RandomIntegerinRange 0 12))
  (bind _returnvalue_3 (Utilities|Select :Index _returnvalue :Option%200 1 :Option%201 2 :Option%202 3 :Option%203 4 :Option%204 5 :Option%205 6 :Option%206 7 :Option%207 8 :Option%208 9 :Option%209 10 :Option%2010 11 :Option%2011 12))
  (bind _returnvalue_4 (Utilities|Select :Index _returnvalue_2 :Option%200 1 :Option%201 2 :Option%202 3 :Option%203 4 :Option%204 5 :Option%205 6 :Option%206 7 :Option%207 8 :Option%208 9 :Option%209 10 :Option%2010 11 :Option%2011 12))
  (Development|PrintString (Utilities|Select :Index (Math|Random|RandomIntegerinRange 0 3) :Option%200 "Diamond" :Option%201 "Heart" :Option%202 "Club" :Option%203 "Spade"))
  (Utilities|Array|Add (Variables|Default|GetPlayer%20Hand) _returnvalue_4)
  (Development|PrintString (Utilities|String|ToString(Integer) _returnvalue_4))
  (Utilities|FlowControl|Delay 1.0)
  (Development|PrintString (Utilities|Select :Index (Math|Random|RandomIntegerinRange 0 3) :Option%200 "Diamond" :Option%201 "Heart" :Option%202 "Club" :Option%203 "Spade") true true "(R=0.000000,G=0.660000,B=1.000000,A=1.000000)" 1e+01)
  (Utilities|Array|Add (Variables|Default|GetDealer%20Hand) _returnvalue_3)
  (Development|PrintString (Utilities|String|Append "Dealer: " (Utilities|String|ToString(Integer) _returnvalue_3)) true true "(R=0.000000,G=0.660000,B=1.000000,A=1.000000)" 1e+01)
  (Utilities|FlowControl|DoOnce false
    (:Completed
      (CallFunction|DealCards))))

(event Custom|CheckForWinorLose
  ;[0.313 1 0.4086 0.5] Checks to See if the player won or lost
  (for _array_element (Variables|Default|GetPlayer%20Hand)
    (bind _output_get (Variables|Default|SetRunning%20Total (+ _array_element (Variables|Default|GetRunning%20Total))))
    (if (>= _output_get 21)
      (Development|PrintString "you lose")
      (elif (== (Variables|Default|GetRunning%20Total) 21)
        (Development|PrintString "you win")
        (elif true
          (Development|PrintString "Hit or stand or double or split"))))))

(event Custom|Hit)

(event EventBeginPlay
  (CallFunction|DealCards))

(fn ConstructionScript)