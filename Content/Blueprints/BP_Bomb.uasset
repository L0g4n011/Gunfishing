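; BP_Bomb is a holdable bomb that the first-person character can pick up, drop and use to trigger explosions on nearby actors.
; Pickup attaches its Sphere to the hand socket with physics and collision off, while Drop re-enables both and teleports it ahead of the camera.
; UseObj waits on a delay, sphere-traces around the bomb with persistent debug drawing, then sends ExplosionMessage to hit actors tagged Explodable.
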(event EventUseObj
  (bind _sphere (Variables|Default|GetSphere))
  (bind _returnvalue (Transformation|GetWorldLocation _sphere))
  (if (not (Variables|Default|GetActivated))
    (Utilities|FlowControl|Delay 5.0)
    (bind _outhits (Collision|MultiSphereTraceForObjects _returnvalue _returnvalue 2.5e+02 (Utilities|Array|MakeArray "ObjectTypeQuery1" "ObjectTypeQuery2" "ObjectTypeQuery3" "ObjectTypeQuery4" "ObjectTypeQuery5" "ObjectTypeQuery6" "ObjectTypeQuery7") false 0 "Persistent"))
    (for _array_element _outhits
      (if (Actor|ActorHasTag (.hitactor _array_element) "Explodable")
        (Utilities|Array|Add (Variables|Default|GetHitObjs) (.hitactor _array_element))))
    (for _array_element_2 (Variables|Default|GetHitObjs)
      (Class|BPIDamage|Explosion(Message) _array_element_2))))

(event EventPickup
  ;[0.15 0.15 0.15 0.5] Copy/paste this for all  held objects
  (bind _asbp_first_person_character (Utilities|Casting|CastToBP_FirstPersonCharacter (Game|GetPlayerCharacter 0)))
  (Transformation|AttachComponentToComponent (Variables|Default|GetSphere) (Variables|/Script/Engine.Character|GetMesh _asbp_first_person_character) "HandGrip_R" "SnapToTarget" "KeepRelative" "KeepRelative" true)
  (Collision|SetActorEnableCollision false)
  (Physics|SetSimulatePhysics (Variables|Default|GetSphere) false))

(event EventDrop
  (bind _returnvalue (Game|GetPlayerCameraManager 0))
  ;[0.15 0.15 0.15 0.5] Copy/paste this for all  held objects
  (Transformation|DetachFromComponent (Variables|Default|GetDefaultSceneRoot) "KeepWorld" "KeepWorld" "KeepWorld" false)
  (Physics|SetSimulatePhysics (Variables|Default|GetSphere) true)
  (Collision|SetActorEnableCollision true)
  (Transformation|SetActorLocation (+ (Camera|GetCameraLocation _returnvalue) (* 75.0 (Transformation|GetActorForwardVector _returnvalue))) false true)
  (Rendering|SetActorHiddenInGame false))

(fn ConstructionScript)