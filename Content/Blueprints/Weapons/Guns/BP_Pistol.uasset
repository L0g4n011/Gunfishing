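; Pistol actor that the player can pick up, drop and fire as a held object.
; Pickup attaches its Cube to the first-person character's right-hand grip socket and disables physics and collision; Drop restores both and places it in front of the camera.
; UseObj fires a debug-drawn Visibility line trace from the Scene component along camera forward, sending ShotMessage with damage to hit actors tagged Shootable.
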(event EventDrop
  (bind _returnvalue (Game|GetPlayerCameraManager 0))
  ;[0.15 0.15 0.15 0.5] Copy/paste this for all  held objects
  (Transformation|DetachFromComponent (Variables|Default|GetDefaultSceneRoot) "KeepWorld" "KeepWorld" "KeepWorld" false)
  (Physics|SetSimulatePhysics (Variables|Default|GetCube) true)
  (Collision|SetActorEnableCollision true)
  (Transformation|SetActorLocation (+ (Camera|GetCameraLocation _returnvalue) (* 75.0 (Transformation|GetActorForwardVector _returnvalue))) false true)
  (Rendering|SetActorHiddenInGame false))

(event EventPickup
  ;[0.15 0.15 0.15 0.5] Copy/paste this for all  held objects
  (bind _asbp_first_person_character (Utilities|Casting|CastToBP_FirstPersonCharacter (Game|GetPlayerCharacter 0)))
  (Transformation|AttachComponentToComponent (Variables|Default|GetCube) (Variables|/Script/Engine.Character|GetMesh _asbp_first_person_character) "HandGrip_R" "SnapToTarget" "KeepRelative" "KeepRelative" true)
  (Collision|SetActorEnableCollision false)
  (Physics|SetSimulatePhysics (Variables|Default|GetCube) false))

(event EventUseObj
  (bind _scene (Variables|Default|GetScene))
  (bind _returnvalue (Transformation|GetWorldLocation _scene))
  (bind (_outhit _returnvalue_2) (Collision|LineTraceByChannel _returnvalue (+ _returnvalue (* (Transformation|GetActorForwardVector (Game|GetPlayerCameraManager 0)) 1e+04)) "TraceTypeQuery1" false 0 "ForDuration"))
  (if _returnvalue_2
    (if (Actor|ActorHasTag (.hitactor _outhit) "Shootable")
      (Class|BPIDamage|Shot(Message) (.hitactor _outhit) (Variables|Default|GetDamage)))))

(fn ConstructionScript)