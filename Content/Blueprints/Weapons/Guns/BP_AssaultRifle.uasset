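; BP_AssaultRifle is a holdable gun that the first-person player can pick up, drop and use.
; Pickup attaches the Cylinder mesh to the character's right-hand grip socket and disables collision and physics.
; Drop detaches the root, restores physics and collision, and teleports the gun just ahead of the camera.
; UseChargeObj only draws a debug visibility trace from ShootingPoint along the camera's forward vector, without using the hit.
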(event EventUseChargeObj
  (params (IsPressed :type Boolean))
  (bind _shootingpoint (Variables|Default|GetShootingPoint))
  (bind _returnvalue (Transformation|GetWorldLocation _shootingpoint))
  (Collision|LineTraceByChannel _returnvalue (+ _returnvalue (* (Transformation|GetActorForwardVector (Game|GetPlayerCameraManager 0)) 1e+04)) "TraceTypeQuery1" false 0 "ForDuration"))

(event EventPickup
  ;[0.15 0.15 0.15 0.5] Copy/paste this for all  held objects
  (bind _asbp_first_person_character (Utilities|Casting|CastToBP_FirstPersonCharacter (Game|GetPlayerCharacter 0)))
  (Transformation|AttachComponentToComponent (Variables|Default|GetCylinder) (Variables|/Script/Engine.Character|GetMesh _asbp_first_person_character) "HandGrip_R" "SnapToTarget" "KeepRelative" "KeepRelative" true)
  (Collision|SetActorEnableCollision false)
  (Physics|SetSimulatePhysics (Variables|Default|GetCylinder) false))

(event EventDrop
  (bind _returnvalue (Game|GetPlayerCameraManager 0))
  ;[0.15 0.15 0.15 0.5] Copy/paste this for all  held objects
  (Transformation|DetachFromComponent (Variables|Default|GetDefaultSceneRoot) "KeepWorld" "KeepWorld" "KeepWorld" false)
  (Physics|SetSimulatePhysics (Variables|Default|GetCylinder) true)
  (Collision|SetActorEnableCollision true)
  (Transformation|SetActorLocation (+ (Camera|GetCameraLocation _returnvalue) (* 75.0 (Transformation|GetActorForwardVector _returnvalue))) false true)
  (Rendering|SetActorHiddenInGame false))

(fn ConstructionScript)