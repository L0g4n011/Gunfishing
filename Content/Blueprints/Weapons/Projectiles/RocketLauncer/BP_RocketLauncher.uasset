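; Held rocket launcher weapon that the player can pick up, drop and fire.
; Pickup attaches the Cone component to the first-person character's right hand socket and disables collision and physics.
; Drop detaches the root, restores physics, collision and visibility, and teleports the actor just in front of the camera.
; UseObj spawns a BP_Rocket at the Scene component, aimed along the camera's forward vector.
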(event EventPickup
  ;[0.15 0.15 0.15 0.5] Copy/paste this for all  held objects
  (bind _asbp_first_person_character (Utilities|Casting|CastToBP_FirstPersonCharacter (Game|GetPlayerCharacter 0)))
  (Transformation|AttachComponentToComponent (Variables|Default|GetCone) (Variables|/Script/Engine.Character|GetMesh _asbp_first_person_character) "HandGrip_R" "SnapToTarget" "KeepRelative" "KeepRelative" true)
  (Collision|SetActorEnableCollision false)
  (Physics|SetSimulatePhysics (Variables|Default|GetCone) false))

(event EventDrop
  (bind _returnvalue (Game|GetPlayerCameraManager 0))
  ;[0.15 0.15 0.15 0.5] Copy/paste this for all  held objects
  (Transformation|DetachFromComponent (Variables|Default|GetDefaultSceneRoot) "KeepWorld" "KeepWorld" "KeepWorld" false)
  (Physics|SetSimulatePhysics (Variables|Default|GetCone) true)
  (Collision|SetActorEnableCollision true)
  (Transformation|SetActorLocation (+ (Camera|GetCameraLocation _returnvalue) (* 75.0 (Transformation|GetActorForwardVector _returnvalue))) false true)
  (Rendering|SetActorHiddenInGame false))

(event EventUseObj
  (Game|SpawnActorfromClass "/Game/Blueprints/Weapons/Projectiles/RocketLauncer/BP_Rocket.BP_Rocket_C" (Math|Transform|MakeTransform (Transformation|GetWorldLocation (Variables|Default|GetScene)) (Math|Conversions|RotationFromXVector (Transformation|GetActorForwardVector (Game|GetPlayerCameraManager 0))) "1.000000,1.000000,1.000000") "Undefined" "MultiplyWithRoot" 0 0))

(fn ConstructionScript)