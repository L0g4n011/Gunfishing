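; Rocket launcher projectile that explodes when its Box component begins an overlap, damaging nearby explodable actors.
; Each Tick it repositions the actor slightly ahead of its Cube component along that component's forward vector.
; On overlap, a debug-drawn multi-sphere trace at the Cube collects actors tagged "Explodable".
; The rocket destroys itself and sends each collected actor an ExplosionMessage with damage, location, radius and force.
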(event OnComponentBeginOverlap(Box)
  (params (OverlappedComponent :type Primitive%20Component%20Object%20Reference) (OtherActor :type Actor%20Object%20Reference) (OtherComp :type Primitive%20Component%20Object%20Reference) (OtherBodyIndex :type Integer) (bFromSweep :type Boolean) (SweepResult :type Hit%20Result%20Structure%20%28by%20ref%29))
  (bind _output_get (Variables|Default|SetLocation (Transformation|GetWorldLocation (Variables|Default|GetCube))))
  (bind _outhits (Collision|MultiSphereTraceForObjects _output_get _output_get (Variables|Default|GetRadius) (Utilities|Array|MakeArray "ObjectTypeQuery1" "ObjectTypeQuery2" "ObjectTypeQuery3" "ObjectTypeQuery4" "ObjectTypeQuery5" "ObjectTypeQuery6" "ObjectTypeQuery7") false 0 "ForDuration"))
  (for _array_element _outhits
    (if (Actor|ActorHasTag (.hitactor _array_element) "Explodable")
      (Utilities|Array|Add (Variables|Default|GetHitObjects) (.hitactor _array_element))))
  (Actor|DestroyActor)
  (for _array_element_2 (Variables|Default|GetHitObjects)
    (Class|BPIDamage|Explosion(Message) _array_element_2 (Variables|Default|GetDamage) (Variables|Default|GetLocation) (Variables|Default|GetRadius) (Variables|Default|GetFORCE))))

(event EventTick
  (params (DeltaSeconds :type Float%20%28single-precision%29))
  (bind _cube (Variables|Default|GetCube))
  (Transformation|SetActorLocation (+ (Transformation|GetWorldLocation _cube) (* (Math|Vector|GetForwardVector _cube) 25.0)) false false))

(fn ConstructionScript)