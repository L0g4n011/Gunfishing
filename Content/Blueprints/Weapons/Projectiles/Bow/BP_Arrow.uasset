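; BP_Arrow is a bow projectile that flies in a straight line along the player's view direction.
; On BeginPlay it stores the forward vector of player 0's camera manager.
; Each Tick it moves its Cube component along that vector by ArrowCharge units, which is not scaled by delta time.
; The move does not sweep, and the graph contains no gravity, hit or damage logic.
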(event EventTick
  (params (DeltaSeconds :type Float%20%28single-precision%29))
  (Transformation|SetWorldLocation (Variables|Default|GetCube) (+ (Transformation|GetWorldLocation (Variables|Default|GetCube)) (* (Variables|Default|GetForward%20Vect) (Variables|Default|GetArrowCharge))) false false))

(event EventBeginPlay
  (Variables|Default|SetForward%20Vect (Transformation|GetActorForwardVector (Game|GetPlayerCameraManager 0))))

(fn ConstructionScript)