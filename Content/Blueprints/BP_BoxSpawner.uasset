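; BP_BoxSpawner is a trigger volume that repeatedly spawns BP_TestBass actors while an actor tagged Player is inside it.
; Begin overlap on SpawnActorsTrigger starts a looping one-second timer, and end overlap clears it through StopSpawningActors.
; Each timer tick runs SpawnActorsOverTime, which spawns one actor at a random point within the trigger's own box extent.
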(event OnComponentBeginOverlap(SpawnActorsTrigger)
  (params (OverlappedComponent :type Primitive%20Component%20Object%20Reference) (OtherActor :type Actor%20Object%20Reference) (OtherComp :type Primitive%20Component%20Object%20Reference) (OtherBodyIndex :type Integer) (bFromSweep :type Boolean) (SweepResult :type Hit%20Result%20Structure%20%28by%20ref%29))
  (if (Actor|ActorHasTag OtherActor "Player")
    (bind _returnvalue (Utilities|Time|SetTimerbyEvent (delegate Custom|SpawnActorsOverTime) 1.0 true))))

(event OnComponentEndOverlap(SpawnActorsTrigger)
  (params (OverlappedComponent :type Primitive%20Component%20Object%20Reference) (OtherActor :type Actor%20Object%20Reference) (OtherComp :type Primitive%20Component%20Object%20Reference) (OtherBodyIndex :type Integer))
  (if (Actor|ActorHasTag OtherActor "Player")
    (CallFunction|StopSpawningActors)))

(event Custom|SpawnActorsOverTime
  (bind _spawnactorstrigger (Variables|Default|GetSpawnActorsTrigger))
  (Game|SpawnActorfromClass "/Game/LootTable/BP_TestBass.BP_TestBass_C" (Math|Transform|MakeTransform (Math|Random|RandomPointinBoundingBox (Transformation|GetWorldLocation _spawnactorstrigger) (Variables|/Script/Engine.BoxComponent|GetBoxExtent _spawnactorstrigger)) "0, 0, 0" "1.000000,1.000000,1.000000") "Undefined" "MultiplyWithRoot" 0 0))

(event Custom|Stop%20Spawning%20Actors
  (Utilities|Time|ClearandInvalidateTimerbyHandle (stale OnComponentBeginOverlap(SpawnActorsTrigger) _returnvalue)))

(fn ConstructionScript)