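; BP_TestBass is a test bass fish actor that takes damage from shots and explosions.
; Shot and Explosion events each subtract damage from Health and enable physics simulation on its Sphere once Health reaches zero or below.
; A lethal explosion also spawns a RadialForceActor_Blueprint at the blast location.
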(event EventShot
  (params (Damage :type Float%20%28double-precision%29))
  (Variables|Default|SetHealth (- (Variables|Default|GetHealth) Damage))
  (if (<= (Variables|Default|GetHealth) 0.0)
    (Physics|SetSimulatePhysics (Variables|Default|GetSphere) true)))

(event EventExplosion
  (params (ExplosionDamage :type Float%20%28double-precision%29) (ExplosionLocation :type Vector :default "0, 0, 0") (ExplosionRadius :type Float%20%28double-precision%29) (ExplosionStrength :type Float%20%28double-precision%29))
  (Variables|Default|SetHealth (- (Variables|Default|GetHealth) ExplosionDamage))
  (if (<= (Variables|Default|GetHealth) 0.0)
    (Physics|SetSimulatePhysics (Variables|Default|GetSphere) true)
    (Game|SpawnActorfromClass "/Game/Blueprints/BPIs/RadialForceActor_Blueprint.RadialForceActor_Blueprint_C" (Math|Conversions|ToTransform(Vector) ExplosionLocation) "Undefined" "MultiplyWithRoot" 0 0)))

(fn ConstructionScript)