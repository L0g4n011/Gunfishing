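; BP_Railgun is a charge-up railgun that the first-person character can pick up into the right-hand socket and drop in front of the camera, toggling physics and collision.
; Each pressed UseChargeObj call adds charge; release fires Shoot if charge reaches the threshold, then resets.
; Shoot runs a debug-drawn multi-object line trace along camera forward from FiringPoint, collecting "Shootable" actors into HitFish, which is cleared immediately afterwards without further use.
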(event EventDrop
  (bind _returnvalue (Game|GetPlayerCameraManager 0))
  (Transformation|DetachFromComponent (Variables|Default|GetDefaultSceneRoot) "KeepWorld" "KeepWorld" "KeepWorld" false)
  (Physics|SetSimulatePhysics (Variables|Default|GetCube) true)
  (Collision|SetActorEnableCollision true)
  (Transformation|SetActorLocation (+ (Camera|GetCameraLocation _returnvalue) (* 75.0 (Transformation|GetActorForwardVector _returnvalue))) false true))

(event EventPickup
  (bind _asbp_first_person_character (Utilities|Casting|CastToBP_FirstPersonCharacter (Game|GetPlayerCharacter 0)))
  (Transformation|AttachComponentToComponent (Variables|Default|GetCube) (Variables|/Script/Engine.Character|GetMesh _asbp_first_person_character) "HandGrip_R" "SnapToTarget" "KeepRelative" "KeepRelative" true)
  (Collision|SetActorEnableCollision false)
  (Physics|SetSimulatePhysics (Variables|Default|GetCube) false))

(event EventUseChargeObj
  (params (IsPressed :type Boolean))
  (if IsPressed
    (bind _output_get (Variables|Default|SetCharge (+ 0.01 (Variables|Default|GetCharge))))
    (Development|PrintString (Utilities|String|ToString(Float) _output_get))
    (else
      (if (>= (Variables|Default|GetCharge) 0.75)
        (CallFunction|Shoot))
      (Variables|Default|SetCharge 0.0)
      (Utilities|Array|Clear (Variables|Default|GetHitFish)))))

(fn ConstructionScript)

(fn Shoot
  (bind _firingpoint (Variables|Default|GetFiringPoint))
  (bind _returnvalue (Transformation|GetWorldLocation _firingpoint))
  (bind _outhits (Class|KismetSystemLibrary|LineTraceMultiforObjects _returnvalue (+ _returnvalue (* (Transformation|GetActorForwardVector (Game|GetPlayerCameraManager 0)) 1e+04)) (Utilities|Array|MakeArray "ObjectTypeQuery1" "ObjectTypeQuery2" "ObjectTypeQuery3" "ObjectTypeQuery4" "ObjectTypeQuery5" "ObjectTypeQuery6" "ObjectTypeQuery7") false 0 "ForDuration" true))
  (for _array_element _outhits
    (if (Actor|ActorHasTag (.hitactor _array_element) "Shootable")
      (Utilities|Array|Add (Variables|Default|GetHitFish) (.hitactor _array_element)))))