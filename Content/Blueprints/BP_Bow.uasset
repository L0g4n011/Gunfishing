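; BP_Bow is a held bow item that the first-person player can pick up, drop and charge to fire arrows.
; Pickup snaps the Cube to the character's hand socket with physics and collision off; Drop restores both and places the bow ahead of the camera.
; UseChargeObj builds a capped ArrowCharge while pressed, then on release spawns a BP_Arrow at ShootingPoint with camera rotation, passes it the charge and resets.
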(event Custom|Shoot
  (bind _returnvalue (Game|SpawnActorfromClass "/Game/Blueprints/BP_Arrow.BP_Arrow_C" (Math|Transform|MakeTransform (Transformation|GetWorldLocation (Variables|Default|GetShootingPoint)) (Camera|GetCameraRotation (Game|GetPlayerCameraManager 0)) "1.000000,1.000000,1.000000") "Undefined" "MultiplyWithRoot" 0 0))
  (Variables|/Game/Blueprints/BP_Arrow.BP_Arrow_C|SetArrowCharge _returnvalue (Variables|Default|Getarrow%20charge%20)))

(event EventUseChargeObj
  (params (IsPressed :type Boolean))
  (if IsPressed
    (if (< (Variables|Default|Getarrow%20charge%20) 1e+01)
      (Variables|Default|Setarrow%20charge%20 (+ (Variables|Default|Getarrow%20charge%20) 0.1)))
    (else
      (CallFunction|Shoot)
      (Variables|Default|Setarrow%20charge%20 0.0))))

(event EventPickup
  ;[0.15 0.15 0.15 0.5] Copy/paste this for all  held objects
  (bind _asbp_first_person_character (Utilities|Casting|CastToBP_FirstPersonCharacter (Game|GetPlayerCharacter 0)))
  (Transformation|AttachComponentToComponent (Variables|Default|GetCube) (Variables|/Script/Engine.Character|GetMesh _asbp_first_person_character) "HandGrip_R" "SnapToTarget" "KeepRelative" "KeepRelative" true)
  (Collision|SetActorEnableCollision false)
  (Physics|SetSimulatePhysics (Variables|Default|GetCube) false))

(event EventDrop
  (bind _returnvalue (Game|GetPlayerCameraManager 0))
  ;[0.15 0.15 0.15 0.5] Copy/paste this for all  held objects
  (Transformation|DetachFromComponent (Variables|Default|GetDefaultSceneRoot) "KeepWorld" "KeepWorld" "KeepWorld" false)
  (Physics|SetSimulatePhysics (Variables|Default|GetCube) true)
  (Collision|SetActorEnableCollision true)
  (Transformation|SetActorLocation (+ (Camera|GetCameraLocation _returnvalue) (* 75.0 (Transformation|GetActorForwardVector _returnvalue))) false true)
  (Rendering|SetActorHiddenInGame false))

(fn ConstructionScript)